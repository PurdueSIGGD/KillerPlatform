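; Spring actor that launches whatever hits it by adding physics velocity along its rotation's Z axis.
; On Hit, the other actor's vertical speed picks the launch speed: a fixed minimum, a reversed and amplified bounce, or a fixed cap, all scaled by SpringFactor.
; The impulse goes to the first PrimitiveComponent found, with a debug print if the cast fails.
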(event `self.ReceiveHit`
  (params (MyComp :type "PrimitiveComponent Object Reference") (Other :type "Actor Object Reference") (OtherComp :type "PrimitiveComponent Object Reference") (bSelfMoved :type Boolean) (HitLocation :type "Object.Vector Structure") (HitNormal :type "Object.Vector Structure") (NormalImpulse :type "Object.Vector Structure") (Hit :type "EngineTypes.HitResult Structure (by ref)"))
  (bind _springfactor (`self.SpringFactor`))
  (bind _z (.z (`self.GetVelocity` Other)))
  (bind _returnvalue (`KismetMathLibrary.Abs` _z))
  (if (>= _returnvalue 600.0)
    (if (<= _returnvalue 2000.0)
      (set `self.LaunchSpeed` (* -1.5 _z _springfactor))
      (else
        (set `self.LaunchSpeed` (* _springfactor 2500.0))))
    (else
      (set `self.LaunchSpeed` (* _springfactor 905.0))))
  (bind _asprimitivecomponent (cast `PrimitiveComponent` (`KismetArrayLibrary.Array_Get` (`self.K2_GetComponentsByClass` Other "/Script/Engine.PrimitiveComponent")))
    (:`then`
      (`PrimitiveComponent.SetPhysicsLinearVelocity` _asprimitivecomponent (* (`.Z` (`KismetMathLibrary.BreakRotIntoAxes` (`self.K2_GetActorRotation`))) (`self.LaunchSpeed`)) true "None"))
    (:`CastFailed`
      (`KismetSystemLibrary.PrintString` "Nothin happened" true true (struct :`R` 1.0 :`B` 0.060021 :`A` 1.0)))))

(fn `NewFunction_0`)

(fn `UserConstructionScript`)