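; A pickup particle that drifts toward the player and is collected on overlap.
; A looping timer, set in both BeginPlay and the construction script, repeatedly adds a velocity-change impulse to ParticlePart, proportional to its offset from the player pawn.
; Overlap with the player's class casts to KillerPlatformCharacter and switches on Itemtype, but all five cases only destroy the actor and play the pickup sound at the world origin.
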(event `self.ReceiveBeginPlay`
  (`KismetSystemLibrary.K2_SetTimer` null "custom_timer" 0.02 true))

(event `custom_timer`
  (`PrimitiveComponent.AddImpulse` (`self.ParticlePart`) (* (- (`self.K2_GetActorLocation` (`GameplayStatics.GetPlayerPawn` 0)) (`self.K2_GetActorLocation`)) 0.05) "None" true))

(event `self.ReceiveActorBeginOverlap`
  (params (OtherActor :type "Actor Object Reference"))
  (if (== (`GameplayStatics.GetObjectClass` OtherActor) (`GameplayStatics.GetObjectClass` (`GameplayStatics.GetPlayerPawn` 0)))
    ;[1 1 1] Switch on the item value, changes int value of the player
    (cast `/Game/Blueprints/KillerPlatformCharacter` OtherActor)
    (switch `int` (`self.itemtype`)
      (:`0`
        _)
      (:`1`
        _)
      (:`2`
        _)
      (:`3`
        _)
      (:`4`
        _))
    (`self.K2_DestroyActor`)
    (`GameplayStatics.PlaySoundAtLocation` "/Game/Audio/chiptune_sounds/pickup.pickup")))

(fn `UserConstructionScript`
  (`KismetSystemLibrary.K2_SetTimer` null "custom_timer" 0.02 true)
  (`KismetSystemLibrary.K2_UnPauseTimer` null "movement"))