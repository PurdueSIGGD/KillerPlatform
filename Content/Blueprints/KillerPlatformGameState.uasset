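; Game state that moves to the next level once all enemies present at the start have been killed.
; The construction script counts Enemy actors, starts the polling and delay timers, and creates a hidden Hotbar widget.
; A looping check compares kills to that count, then unpauses the delay and plays the victory sound on every poll until GoOn is set.
; NumEnemiesKilled is only reset here, never incremented.
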(event `newmapcheck`
  ;[1 1 1] Opening a new level
  (if (>= (`self.NumEnemiesKilled`) (`self.NumInitialEnemies`))
    (if (`self.go on`)
      (`KismetSystemLibrary.K2_PauseTimer` null "newmapdelay")
      (`GameplayStatics.OpenLevel` (`self.nextLevel`))
      (else
        (`KismetSystemLibrary.K2_UnPauseTimer` null "newmapdelay")
        (`GameplayStatics.PlaySoundAttached` "/Game/Audio/music/victory.victory")))))

(event `newmapdelay`
  ;[1 1 1] Opening a new level
  (set `self.go on` true))

(fn `NewFunction_0`)

(fn `UserConstructionScript`
  (bind _outactors (`GameplayStatics.GetAllActorsOfClass` "/Game/Blueprints/Enemy.Enemy_C"))
  (set `self.NumInitialEnemies` (`KismetArrayLibrary.Array_Length` _outactors))
  (`KismetSystemLibrary.PrintString` (`KismetStringLibrary.Concat_StrStr` "Initial enemies: " (`KismetStringLibrary.Conv_IntToString` (`self.NumInitialEnemies`))))
  (set `self.NumEnemiesKilled` 0)
  (`KismetSystemLibrary.PrintString` (`KismetStringLibrary.Concat_StrStr` "Enemies killed:" (`KismetStringLibrary.Conv_IntToString` (`self.NumEnemiesKilled`))))
  (`KismetSystemLibrary.K2_SetTimer` null "newmapcheck" 0.25 true)
  (`KismetSystemLibrary.K2_SetTimer` null "newmapdelay" 5.0 true)
  (`KismetSystemLibrary.K2_PauseTimer` null "newmapdelay")
  (bind _returnvalue (`|CreateWidget` "/Game/Widgets/Hotbar.Hotbar_C"))
  (`UserWidget.AddToViewport` _returnvalue)
  (`Widget.SetVisibility` _returnvalue "Hidden")
  (set `self.hotbar1` _returnvalue))