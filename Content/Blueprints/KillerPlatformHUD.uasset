(event `self.ReceiveDrawHUD`
  (params (SizeX :type Integer) (SizeY :type Integer))
  (bind _returnvalue (* SizeY 0.05))
  (bind _returnvalue_2 (* SizeX 0.9))
  (bind _textcolor (`self.TextColor`))
  (bind _askillerplatformgamestate_c (cast `/Game/Blueprints/KillerPlatformGameState` (`GameplayStatics.GetGameState`)))
  (bind _numenemieskilled (`/Game/Blueprints/KillerPlatformGameState.NumEnemiesKilled` _askillerplatformgamestate_c))
  (bind _numinitialenemies (`/Game/Blueprints/KillerPlatformGameState.NumInitialEnemies` _askillerplatformgamestate_c))
  (if (>= _numenemieskilled _numinitialenemies)
    (`self.DrawText` "You Win!" _textcolor _returnvalue_2 _returnvalue)
    (else
      (`self.DrawText` (`KismetStringLibrary.Concat_StrStr` (`KismetStringLibrary.Concat_StrStr` (`KismetStringLibrary.Concat_StrStr` "Killed: " (`KismetStringLibrary.Conv_IntToString` _numenemieskilled)) "/") (`KismetStringLibrary.Conv_IntToString` _numinitialenemies)) _textcolor _returnvalue_2 _returnvalue))))

(fn `UserConstructionScript`)