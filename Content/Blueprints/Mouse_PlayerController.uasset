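; Player controller that places items with the mouse in the Killer Platform game.
; On left click it reads PlacingItem from the game state, and the only handled item spawns a SpringActor before resetting that value to zero.
; The spawn point is the deprojected cursor position, nudged along the view direction, with Y zeroed to keep it on the XZ plane.
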(event `Key|LeftMouseButton`
  (bind (_worldlocation _worlddirection) (`self.DeprojectMousePositionToWorld`))
  (bind _returnvalue (+ _worldlocation (* _worlddirection 1.0)))
  (:`Pressed`
    (bind _askillerplatformgamestate_c (cast `/Game/Blueprints/KillerPlatformGameState` (`GameplayStatics.GetGameState`)))
    (switch `int` (`/Game/Blueprints/KillerPlatformGameState.placingItem` _askillerplatformgamestate_c)
      (:`1`
        (set `self.mousePos` (- _returnvalue (`KismetMathLibrary.MakeVector` 0.0 (.y _returnvalue))))
        (`|SpawnActorFromClass` "/Game/Blueprints/SpringActor.SpringActor_C" (`KismetMathLibrary.Conv_VectorToTransform` (`self.mousePos`)))
        (set `/Game/Blueprints/KillerPlatformGameState.placingItem` 0 _askillerplatformgamestate_c)))))

(fn `UserConstructionScript`)