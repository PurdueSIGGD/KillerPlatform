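; KillerPlatformHUD is a HUD Blueprint that switches drawing between a main menu screen and a game screen.
; On BeginPlay it spawns a GameMenuScreen actor and a GameScreen actor and keeps references to both.
; Each DrawHUD call stores the screen size, then switches on ScreenType to send the matching screen its message, delegating per-screen work to those actors.
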(event `self.ReceiveBeginPlay`
  (bind _returnvalue (`|SpawnActorFromClass` "/Game/Blueprints/HUD/GameMenuScreen.GameMenuScreen_C" (`self.Null Transform`)))
  (set `self.MainMenu` _returnvalue)
  (bind _returnvalue_2 (`|SpawnActorFromClass` "/Game/Blueprints/HUD/GameScreen.GameScreen_C" (`self.NullTransform`)))
  (set `self.GameScreen` _returnvalue_2))

(event `self.ReceiveDrawHUD`
  (params (SizeX :type Integer) (SizeY :type Integer))
  (set `self.ScreenSize` (`KismetMathLibrary.MakeVector2D` (`KismetMathLibrary.Conv_IntToDouble` SizeX) (`KismetMathLibrary.Conv_IntToDouble` SizeY)))
  (switch `/Game/Blueprints/HUD/ScreenEnum` (`self.ScreenType`)
    (:`NewEnumerator0`
      (message `/Game/Blueprints/HUD/ScreensInterface.MainMenuScreen` (`self.MainMenu`)))
    (:`NewEnumerator5`
      (message `/Game/Blueprints/HUD/ScreensInterface.GameScreen` (`self.GameScreen`)))))

(fn `UserConstructionScript`)