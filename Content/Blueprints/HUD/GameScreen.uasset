(event `self.GameScreen`
  (bind _returnvalue (* 0 0.05))
  (bind _returnvalue_2 (* 0 0.9))
  (bind _textcolor (`self.TextColor`))
  (bind _askillerplatformgamestate_c (cast `/Game/Blueprints/KillerPlatformGameState` (`GameplayStatics.GetGameState`)))
  (bind _numenemieskilled (`/Game/Blueprints/KillerPlatformGameState.NumEnemiesKilled` _askillerplatformgamestate_c))
  (bind _numinitialenemies (`/Game/Blueprints/KillerPlatformGameState.NumInitialEnemies` _askillerplatformgamestate_c))
  (if (>= _numenemieskilled _numinitialenemies)
    (`HUD.DrawText` (`self.WinScreen`) "You Win!" _textcolor _returnvalue_2 _returnvalue null 1.0 false)
    (set `self.counterActive` true)
    (else
      (`HUD.DrawText` (`self.LoseScreen`) (`KismetStringLibrary.Concat_StrStr` (`KismetStringLibrary.Concat_StrStr` (`KismetStringLibrary.Concat_StrStr` "Killed: " (`KismetStringLibrary.Conv_IntToString` _numenemieskilled)) "/") (`KismetStringLibrary.Conv_IntToString` _numinitialenemies)) _textcolor _returnvalue_2 _returnvalue null 1.0 false))))

(fn `UserConstructionScript`)