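; KillerPlatformDefaultHUD is a HUD Blueprint sketched to manage a main menu screen and a game screen, but it is currently inert.
; BeginPlay and DrawHUD are empty, and the construction script does nothing.
; Disconnected nodes would spawn both screens as actors, store the screen size, and call the main menu's message by ScreenType.
; The game screen's message call is also orphaned, separate from that switch.
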(event `self.ReceiveBeginPlay`)

(event `self.ReceiveDrawHUD`
  (params (SizeX :type Integer) (SizeY :type Integer)))

(fn `UserConstructionScript`)