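; ToggleLever is a 2D sprite lever that the player toggles with the L key while manipulation is allowed by overlap.
; Any overlap enables it, as that class check is disconnected; only KillerPlatformCharacter leaving disables it.
; Toggling swaps the on/off sprite and hides ActorToControl without collision when on, restoring both when off.
; Each toggle also applies a zero impulse to Enemy actors cast to PaperSpriteActor.
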(event `self.ReceiveBeginPlay`
  (`self.EnableInput` (`GameplayStatics.GetPlayerController` 0)))

(event `self.ReceiveActorBeginOverlap`
  (params (OtherActor :type "Actor Object Reference"))
  (set `self.CanManipulate` true))

(event `self.ReceiveActorEndOverlap`
  (params (OtherActor :type "Actor Object Reference"))
  (if (== (`GameplayStatics.GetObjectClass` (stale `self.ReceiveActorBeginOverlap` OtherActor)) "/Game/Blueprints/KillerPlatformCharacter.KillerPlatformCharacter_C")
    (set `self.CanManipulate` false)))

(event `Key|L`
  (:`Pressed`
    (if (`self.CanManipulate`)
      (`self.LeverToggled`))))

(fn `LeverToggled`
  (bind _sprite (`self.Sprite`))
  (bind _leverstate (`self.LeverState`))
  (bind _actortocontrol (`self.ActorToControl`))
  (set `self.LeverState` (not (`self.LeverState`)))
  (if _leverstate
    (`PaperSpriteComponent.SetSprite` _sprite (`self.SpriteOn`))
    (else
      (`PaperSpriteComponent.SetSprite` _sprite (`self.SpriteOff`))))
  (`self.SetActorEnableCollision` _actortocontrol (not _leverstate))
  (`self.SetActorHiddenInGame` _actortocontrol _leverstate)
  (bind _outactors (`GameplayStatics.GetAllActorsOfClass` "/Game/Blueprints/Enemy.Enemy_C"))
  (for _array_element _outactors
    (bind _aspaperspriteactor (cast `PaperSpriteActor` _array_element))
    (`PrimitiveComponent.AddImpulse` _aspaperspriteactor (0.0 0.0 0.0) "None" false)))

(fn `UserConstructionScript`
  (`PaperSpriteComponent.SetSprite` (`self.Sprite`) (`self.SpriteOff`))
  (set `self.LeverState` false))