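; A 2D Paper sprite ledge that wears down while another actor overlaps it, then breaks and falls.
; A fast looping timer feeds a Gate that overlap begin and end open and close, draining Health each tick it is open.
; Below zero Health it swaps to the broken sprite, simulates physics, disables collision and plays a fall sound.
; Intermediate damage thresholds are empty, and BeginPlay also sets the broken sprite.
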(event `self.ReceiveBeginPlay`
  (`KismetSystemLibrary.K2_SetTimer` null "breakingstuff" 0.02 true)
  (`PaperSpriteComponent.SetSprite` (`self.PaperSprite1`) "/Game/Sprites/platformBroken_Sprit.platformBroken_Sprit"))

(event `breakingstuff`
  (bind _health (`self.Health`))
  (if (not (`self.Broken`))
    (`/Engine/EditorBlueprintResources/StandardMacros.Gate` true :!label _label
      (:`Exit`
        (set `self.Health` (- _health 1))
        ;[1 1 1] Sample damage states
        (if (< _health 0)
          (`PaperSpriteComponent.SetSprite` (`self.PaperSprite1`) "/Game/Sprites/platformBroken_Sprit.platformBroken_Sprit")
          (`self.K2_SetActorLocation` (`KismetMathLibrary.MakeVector` (.x (`self.K2_GetActorLocation`)) (- (.y (`self.K2_GetActorLocation`)) 0.0) (.z (`self.K2_GetActorLocation`))) true)
          (`PrimitiveComponent.SetSimulatePhysics` (`self.PaperSprite1`) true)
          (`self.SetActorEnableCollision` false)
          (`GameplayStatics.PlaySoundAtLocation` "/Game/Audio/chiptune_sounds/platform_fall_cue.platform_fall_cue")
          (set `self.Broken` true)
          (elif (< _health 25)
            _
            (elif (< _health 50)
              _
              (elif (< _health 75)
                _))))))))

(event `self.ReceiveActorBeginOverlap`
  (params (OtherActor :type "Actor Object Reference"))
  (if (!= (`GameplayStatics.GetObjectClass` OtherActor) "DestructibleLedge_C")
    (goto _label :!via `Open`)))

(event `self.ReceiveActorEndOverlap`
  (params (OtherActor :type "Actor Object Reference"))
  (goto _label :!via `Close`))

(fn `UserConstructionScript`
  (`parent.UserConstructionScript`))