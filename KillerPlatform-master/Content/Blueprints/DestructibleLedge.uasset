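; DestructibleLedge is a Paper2D ledge that crumbles a short time after it is first hit.
; A Hit event starts a countdown, and Tick drains Health by one per frame, so the delay depends on frame rate.
; Once Health drops below zero, it swaps to the second sprite, disables actor collision and stays broken.
; Overlap begin and end only print debug strings.
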(event `self.ReceiveTick`
  (params (DeltaSeconds :type "Float (single-precision)"))
  (bind _health (`self.Health`))
  (if (and (not (`self.Broken`)) (`self.Started`))
    (set `self.Health` (- _health 1))
    (if (< _health 0)
      (`SceneComponent.SetVisibility` (`self.PaperSprite2`) true false)
      (`SceneComponent.SetVisibility` (`self.PaperSprite1`) false false)
      (`self.SetActorEnableCollision` false)
      (set `self.Broken` true))))

(event `self.ReceiveHit`
  (params (MyComp :type "PrimitiveComponent Object Reference") (Other :type "Actor Object Reference") (OtherComp :type "PrimitiveComponent Object Reference") (bSelfMoved :type Boolean) (HitLocation :type "Object.Vector Structure") (HitNormal :type "Object.Vector Structure") (NormalImpulse :type "Object.Vector Structure") (Hit :type "EngineTypes.HitResult Structure (by ref)"))
  (set `self.Started` true))

(event `self.ReceiveActorBeginOverlap`
  (params (OtherActor :type "Actor Object Reference"))
  (`KismetSystemLibrary.PrintString` "Crack crack"))

(event `self.ReceiveActorEndOverlap`
  (params (OtherActor :type "Actor Object Reference"))
  (`KismetSystemLibrary.PrintString` "whew"))

(fn `UserConstructionScript`
  (`parent.UserConstructionScript`))