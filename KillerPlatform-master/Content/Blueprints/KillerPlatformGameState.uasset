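; KillerPlatformGameState is a game state Blueprint that holds a resource count, the initial enemy count and an enemies-killed tally.
; Its Construction Script zeroes the resource and kill counters and sets the initial enemy count by finding all Enemy actors in the world.
; It prints both enemy figures to the screen as debug text.
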(fn `UserConstructionScript`
  (set `self.ResourceCount` 0)
  (bind _outactors (`GameplayStatics.GetAllActorsOfClass` "/Game/Blueprints/Enemy.Enemy_C"))
  (set `self.NumInitialEnemies` (`KismetArrayLibrary.Array_Length` _outactors))
  (`KismetSystemLibrary.PrintString` (`KismetStringLibrary.Concat_StrStr` "Initial enemies: " (`KismetStringLibrary.Conv_IntToString` (`self.NumInitialEnemies`))))
  (set `self.NumEnemiesKilled` 0)
  (`KismetSystemLibrary.PrintString` (`KismetStringLibrary.Concat_StrStr` "Enemies killed:" (`KismetStringLibrary.Conv_IntToString` (`self.NumEnemiesKilled`)))))