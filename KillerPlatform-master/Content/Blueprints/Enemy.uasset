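; Enemy actor that dies when it hits Spikes or is struck hard enough by the KillerPlatformCharacter.
; The Hit event checks the other actor's class and, for the character, compares its component's full velocity magnitude, not just vertical, against MinimumVerticalVelocityToKill.
; EnemyKilled destroys the actor and increments NumEnemiesKilled and ResourceCount on KillerPlatformGameState.
; Debug prints report hits; the construction script and NewFunction_0 are empty.
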(event `self.ReceiveHit`
  (params (MyComp :type "PrimitiveComponent Object Reference") (Other :type "Actor Object Reference") (OtherComp :type "PrimitiveComponent Object Reference") (bSelfMoved :type Boolean) (HitLocation :type "Object.Vector Structure") (HitNormal :type "Object.Vector Structure") (NormalImpulse :type "Object.Vector Structure") (Hit :type "EngineTypes.HitResult Structure (by ref)"))
  (bind _returnvalue (`GameplayStatics.GetObjectClass` Other))
  (`KismetSystemLibrary.PrintString` (`KismetSystemLibrary.GetClassDisplayName` _returnvalue))
  (if (== _returnvalue "/Game/Blueprints/Spikes.Spikes_C")
    (`self.Event Enemy Killed` :!label _label)
    (else
      (bind _returnvalue_2 (`PrimitiveComponent.GetPhysicsLinearVelocity` OtherComp "None"))
      (`KismetSystemLibrary.PrintString` (`KismetStringLibrary.Concat_StrStr` "Hit with velocity: " (`KismetStringLibrary.Conv_VectorToString` _returnvalue_2)))
      (if (== (`GameplayStatics.GetObjectClass` Other) "/Game/Blueprints/KillerPlatformCharacter.KillerPlatformCharacter_C")
        (if (>= (`KismetMathLibrary.VSize` _returnvalue_2) (`self.MinimumVerticalVelocityToKill`))
          (goto _label))))))

(event `Event Enemy Killed`
  ;[1 1 1] When enemy is killed
  (`self.K2_DestroyActor`)
  (bind _askillerplatformgamestate_c (cast `/Game/Blueprints/KillerPlatformGameState` (`GameplayStatics.GetGameState`)))
  (set `/Game/Blueprints/KillerPlatformGameState.NumEnemiesKilled` (+ (`/Game/Blueprints/KillerPlatformGameState.NumEnemiesKilled` _askillerplatformgamestate_c) 1) _askillerplatformgamestate_c)
  (set `/Game/Blueprints/KillerPlatformGameState.ResourceCount` (+ (`/Game/Blueprints/KillerPlatformGameState.ResourceCount` _askillerplatformgamestate_c) 1) _askillerplatformgamestate_c))

(fn `NewFunction_0`)

(fn `UserConstructionScript`)